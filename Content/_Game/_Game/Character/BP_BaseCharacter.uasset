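; BP_BaseCharacter is a base character Blueprint with debug instrumentation for jumps and a stub weapon-fire event.
; Pressing Space records start time and height, then the bound apex event prints elapsed time (mislabeled "Jump to Land time") and height gained.
; Landing prints apex-to-land and total jump times.
; FireWeapon only prints a placeholder message and calls GetCameraLookDirection without using the result.
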(event Custom|ReachedJumpApexEvent
  (Class|BaseCharacter|ReachedJumpApex)
  (bind _output_get (Variables|Default|SetJumpApexTime (Utilities|Time|GetTimeSeconds)))
  (Development|PrintString (Utilities|String|Append "Jump to Land time: " (Utilities|String|ToString(Float) (- _output_get (Variables|Default|GetJumpTime)))))
  (Development|PrintString (Utilities|String|Append "Height:  " (Utilities|String|ToString(Float) (- (.z (Transformation|GetActorLocation)) (Variables|Default|GetJumpZ))))))

(event EventBeginPlay
  (Character|BindEventtoOnReachedJumpApex (delegate Custom|ReachedJumpApexEvent)))

(event EventOnLanded
  (params (Hit :type Hit%20Result%20Structure%20%28by%20ref%29))
  (Development|PrintString (Utilities|String|Append "Apex to Land time: " (Utilities|String|ToString(Float) (- (Utilities|Time|GetTimeSeconds) (Variables|Default|GetJumpApexTime)))))
  (Development|PrintString (Utilities|String|Append "Jump to Land time: " (Utilities|String|ToString(Float) (- (Utilities|Time|GetTimeSeconds) (Variables|Default|GetJumpTime))))))

(event EventFireWeapon
  (Development|PrintString "pew pew")
  (Class|BaseCharacter|GetCameraLookDirection))

(event Input|KeyboardEvents|SpaceBar
  (params (Key :type Key%20Structure :default "None"))
  (:Pressed
    (Variables|Default|SetJumpTime (Utilities|Time|GetTimeSeconds))
    (Variables|Default|SetJumpZ (.z (Transformation|GetActorLocation)))))

(fn ConstructionScript)